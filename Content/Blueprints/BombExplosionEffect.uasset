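; Short-lived bomb explosion effect actor that draws a cross-shaped blast along vertical and horizontal arms.
; On BeginPlay, ExplosionLength takes four per-side lengths from the Direction array and moves the start and end positions of the Vertical and Horizontal components along X, negating the opposite side.
; Each arm can therefore reach a different distance on each side before the actor expires after half a second.
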(event `self.ReceiveBeginPlay`
  (bind _direction (`self.Direction`))
  (`self.ExplosionLength` (`|GetArrayItem` _direction) (`|GetArrayItem` _direction 1) (`|GetArrayItem` _direction 2) (`|GetArrayItem` _direction 3))
  (`self.SetLifeSpan` 0.5))

(fn `ExplosionLength`
  (params (Forward :type "Float (double-precision)") (Backward :type "Float (double-precision)") (Right :type "Float (double-precision)") (Left :type "Float (double-precision)"))
  (`SplineMeshComponent.SetStartPosition` (`self.Vertical`) (`KismetMathLibrary.MakeVector` Forward) true)
  (`SplineMeshComponent.SetEndPosition` (`self.Vertical`) (`KismetMathLibrary.MakeVector` (* Backward -1.0)) true)
  (`SplineMeshComponent.SetStartPosition` (`self.Horizontal`) (`KismetMathLibrary.MakeVector` Right) true)
  (`SplineMeshComponent.SetEndPosition` (`self.Horizontal`) (`KismetMathLibrary.MakeVector` (* Left -1.0)) true))

(fn `UserConstructionScript`)