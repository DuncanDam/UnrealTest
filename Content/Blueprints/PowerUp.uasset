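; Bomberman-style power-up pickup that grants its PowerUpType (extra blast, extra bomb, extra speed or remote control) to a BomberCharacter.
; On BeginPlay, a Billboard shows the sprite matching that type.
; When a BomberCharacter overlaps the Cube, the pickup passes its type to the character's GetPowerUp and expires through a very short life span.
; Any damage also destroys it the same way, without granting the power-up.
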(event `self.ReceiveBeginPlay`
  (`BillboardComponent.SetSprite` (`self.Billboard`) (select `EPowerUpType` (`self.PowerUpType`) :`ExtraBlast` "/Engine/EditorResources/S_Emitter.S_Emitter" :`ExtraBomb` "/Engine/EditorResources/S_PortalActorIcon.S_PortalActorIcon" :`ExtraSpeed` "/Engine/EditorResources/S_Thruster.S_Thruster" :`RemoteControl` "/Engine/EditorResources/S_Player.S_Player" :!type "Texture2D Object Reference")))

(event `self.ReceiveAnyDamage`
  (params (Damage :type "Float (single-precision)") (DamageType :type "DamageType Object Reference") (InstigatedBy :type "Controller Object Reference") (DamageCauser :type "Actor Object Reference"))
  (`self.SetLifeSpan` 0.01))

(event `self.Cube.OnComponentBeginOverlap`
  (params (OverlappedComponent :type "PrimitiveComponent Object Reference") (OtherActor :type "Actor Object Reference") (OtherComp :type "PrimitiveComponent Object Reference") (OtherBodyIndex :type Integer) (bFromSweep :type Boolean) (SweepResult :type "HitResult Structure (by ref)"))
  (bind _asbomber_character (cast `BomberCharacter` OtherActor))
  (`BomberCharacter.GetPowerUp` _asbomber_character (`self.PowerUpType`))
  (`self.SetLifeSpan` 0.01))

(fn `UserConstructionScript`)