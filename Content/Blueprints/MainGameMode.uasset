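; MainGameMode is a game mode that owns the main UI and switches the player to menu input at match start and end.
; On BeginPlay it creates MainUI with a reference to itself, adds it to the viewport, and gives player 0 UI-only input with a visible cursor.
; When the match ends, it passes the winning team to MainUI and applies the same cursor and input setup.
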(event `self.ReceiveBeginPlay`
  (bind _returnvalue (`GameplayStatics.GetPlayerController` 0))
  (bind _returnvalue_2 (`|CreateWidget` "/Game/Blueprints/MainUI.MainUI_C" null self))
  (bind _output_get (set `self.MainUI` _returnvalue_2))
  (`UserWidget.AddToViewport` _output_get 0)
  (`WidgetBlueprintLibrary.SetInputMode_UIOnlyEx` _returnvalue (`self.MainUI`))
  (set `PlayerController.bShowMouseCursor` true _returnvalue))

(event `self.OnEndMatch`
  (bind _returnvalue (`GameplayStatics.GetPlayerController` 0))
  (`/Game/Blueprints/MainUI.OnEndMatch` (`self.MainUI`) (`self.GetWinnerTeam`))
  (set `PlayerController.bShowMouseCursor` true _returnvalue)
  (`WidgetBlueprintLibrary.SetInputMode_UIOnlyEx` _returnvalue (`self.MainUI`)))

(fn `UserConstructionScript`)