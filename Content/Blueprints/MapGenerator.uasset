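; Map generator actor that builds a block-grid level from MapData once its OnInitDone event fires.
; The floor and four border walls are scaled instances in the Surrounding instanced mesh, sized from the map dimensions.
; Indestructible blocks become instances of a second instanced mesh, while each destructible block spawns its own actor carrying its block data.
; Each pass clears previous instances and destroys previously spawned walls before rebuilding.
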(event `self.OnInitDone`
  (`self.CreateSurroundingWall`)
  (`self.CreateIndestructibleWalls`)
  (`self.CreateDestructibleWalls`))

(fn `CreateDestructibleWalls`
  (for _array_element (`self.DestructibleWalls`)
    (`/Engine/EditorBlueprintResources/StandardMacros.IsValid` _array_element
      (:`Is Valid`
        (`self.K2_DestroyActor` _array_element))))
  (`KismetArrayLibrary.Array_Clear` (`self.DestructibleWalls`))
  (for _array_element_2 (`.Blocks` (break `MapData` (`self.MapData`)))
    (bind (_x _y _blocktype _location) (break `MapBlock` _array_element_2))
    (if (`|EnumEquality` _blocktype "Destructible")
      (bind _returnvalue (`|SpawnActorFromClass` "/Game/Blueprints/DestructibelWall.DestructibelWall_C" (`KismetMathLibrary.MakeTransform` _location) "AlwaysSpawn" "OverrideRootScale" null _array_element_2 null))
      (`KismetArrayLibrary.Array_Add` (`self.DestructibleWalls`) _returnvalue))))

(fn `CreateIndestructibleWalls`
  (locals (XIndex :type Integer) (YIndex :type Integer))
  (`InstancedStaticMeshComponent.ClearInstances` (`self.IndestructibleWall`))
  (for _array_element (`.Blocks` (break `MapData` (`self.MapData`)))
    (bind (_x _y _blocktype _location) (break `MapBlock` _array_element))
    (if (`|EnumEquality` _blocktype "Indestructible")
      (`InstancedStaticMeshComponent.AddInstance` (`self.IndestructibleWall`) (`KismetMathLibrary.MakeTransform` _location)))))

(fn `CreateSurroundingWall`
  (locals (MeshTransform :type "Array of Transform Structure"))
  (bind (_sizewidth _sizelength _width _length _blocksize) (break `MapData` (`self.MapData`)))
  (bind (_sizewidth_2 _sizelength_2 _width_2 _length_2 _blocksize_2) (break `MapData` (`self.MapData`)))
  (bind (_sizewidth_3 _sizelength_3 _width_3 _length_3 _blocksize_3) (break `MapData` (`self.MapData`)))
  (bind _returnvalue (`KismetMathLibrary.Conv_IntToDouble` _sizelength))
  (bind _returnvalue_2 (/ (- _length _blocksize) -2.0))
  (bind _returnvalue_3 (/ (- _width_3 _blocksize_3) 2.0))
  (bind _returnvalue_4 (`KismetMathLibrary.Conv_IntToDouble` (+ _sizewidth_3 2)))
  (`InstancedStaticMeshComponent.ClearInstances` (`self.Surrounding`))
  ;[1 1 1] Floor Transform
  (`InstancedStaticMeshComponent.AddInstance` (`self.Surrounding`) (`KismetMathLibrary.MakeTransform` (`KismetMathLibrary.MakeVector` (/ (- _length_2 _blocksize_2) -2.0) (/ (- _width_2 _blocksize_2) 2.0) (* _blocksize_2 -1.0)) (struct) (`KismetMathLibrary.MakeVector` (`KismetMathLibrary.Conv_IntToDouble` _sizelength_2) (`KismetMathLibrary.Conv_IntToDouble` _sizewidth_2) 1.0)))
  ;[1 1 1] Top And Bot Transfrom
  (`InstancedStaticMeshComponent.AddInstance` (`self.Surrounding`) (`KismetMathLibrary.MakeTransform` (`KismetMathLibrary.MakeVector` _blocksize_3 _returnvalue_3) (struct) (`KismetMathLibrary.MakeVector` 1.0 _returnvalue_4 1.0)))
  (`InstancedStaticMeshComponent.AddInstance` (`self.Surrounding`) (`KismetMathLibrary.MakeTransform` (`KismetMathLibrary.MakeVector` (- 0.0 _length_3) _returnvalue_3) (struct) (`KismetMathLibrary.MakeVector` 1.0 _returnvalue_4 1.0)))
  ;[1 1 1] Left and Right Transfrom
  (`InstancedStaticMeshComponent.AddInstance` (`self.Surrounding`) (`KismetMathLibrary.MakeTransform` (`KismetMathLibrary.MakeVector` _returnvalue_2 (- 0.0 _blocksize)) (struct) (`KismetMathLibrary.MakeVector` _returnvalue 1.0 1.0)))
  (`InstancedStaticMeshComponent.AddInstance` (`self.Surrounding`) (`KismetMathLibrary.MakeTransform` (`KismetMathLibrary.MakeVector` _returnvalue_2 _width) (struct) (`KismetMathLibrary.MakeVector` _returnvalue 1.0 1.0))))

(fn `UserConstructionScript`)