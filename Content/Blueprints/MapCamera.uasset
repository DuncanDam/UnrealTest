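; MapCamera is the shared match camera for an Unreal Bomberman game, taking over player 0's view on BeginPlay.
; While a match runs, Tick places it near the generated map's middle with a slight X offset.
; It smoothly zooms the spring arm as bombers spread from the center, lerping between a base length and the map's larger dimension via FInterpTo.
; GetMapMiddle and the construction script are empty.
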(event `self.ReceiveBeginPlay`
  (`PlayerController.SetViewTargetWithBlend` (`GameplayStatics.GetPlayerController` 0) self 0.0 "VTBlend_Linear" 0.0 false))

(event `self.ReceiveTick`
  (params (DeltaSeconds :type "Float (single-precision)"))
  (bind _springarm (`self.SpringArm`))
  (set `self.Delta` DeltaSeconds)
  (bind _gamemode (`self.GetGameMode`)
    (:`Out`
      ;[1 1 1] Zoom Control based on distance of player to center
      (bind _output_get (set `self.GameMode` _gamemode))
      (if (`GameMode.IsMatchInProgress` _output_get)
        (`|ExecutionSequence`
          (:`then_0`
            (`self.K2_SetActorLocation` (+ (`.MiddlePoint` (break `MapData` (`MapGenerator.MapData` (`UnrealBombermanGameMode.GetMapGenerator` (`self.GameMode`))))) (50.0 0.0 0.0))))
          (:`then_1`
            (bind _maxrange (`self.GetCameraRange`))
            (set `SpringArmComponent.TargetArmLength` (`KismetMathLibrary.FInterpTo` (`SpringArmComponent.TargetArmLength` _springarm) (`KismetMathLibrary.Lerp` 1000.0 _maxrange (/ (`UnrealBombermanGameMode.GetBombersMaxDistToCenter` (`self.GameMode`)) (/ _maxrange 2.0))) (`self.Delta`) 10.0) _springarm)))))))

(fn `GetCameraRange`
  (returns (MaxRange :type "Float (double-precision)"))
  (bind _gamemode (`self.GetGameMode`)
    (:`Out`
      (bind (_sizewidth _sizelength _width _length) (break `MapData` (`MapGenerator.MapData` (`UnrealBombermanGameMode.GetMapGenerator` _gamemode))))
      (return (`KismetMathLibrary.FMax` _width _length 1000.0)))))

(fn `GetMapMiddle`)

(fn `UserConstructionScript`)